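; BP_Level is an interactive lever that opens and closes a linked gate when the player uses it.
; A collision overlap flags when the first-person character is in range, and the Interact input, enabled at BeginPlay, works only then.
; Each press alternates between opening and closing Mygate, while a timeline plays or reverses to lerp the lever cube's rotation between two rotators.
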(event `self.ReceiveBeginPlay`
  (`self.EnableInput` (`GameplayStatics.GetPlayerController` 0)))

(event `InputAction|Interact` :consume false
  (params (Key :type "Key Structure"))
  (:`Pressed`
    (if (`self.Itsinthezone`)
      (if (`self.ActivateMechanism`)
        (`/Game/1-NOTDoom-Folder/BP_Gate.OpenDoor` (`self.Mygate`))
        (set `self.ActivateMechanism` false)
        (bind (_direction _dooropening) (`Timeline|Línea de tiempo_0` :!label _label)
          (:`Update`
            (`SceneComponent.K2_SetRelativeRotation` (`self.Levercube`) (`KismetMathLibrary.RLerp` (`self.Mystartposition`) (`self.MyMovement`) _dooropening) false false)))
        (else
          (`/Game/1-NOTDoom-Folder/BP_Gate.Close the door` (`self.Mygate`))
          (set `self.ActivateMechanism` true)
          (goto _label :!via `Reverse`))))))

(event `self.LevelCollision.OnComponentBeginOverlap`
  (params (OverlappedComponent :type "PrimitiveComponent Object Reference") (OtherActor :type "Actor Object Reference") (OtherComp :type "PrimitiveComponent Object Reference") (OtherBodyIndex :type Integer) (bFromSweep :type Boolean) (SweepResult :type "HitResult Structure (by ref)"))
  (cast `/Game/FirstPerson/Blueprints/BP_FirstPersonCharacter` OtherActor)
  (set `self.Itsinthezone` true))

(event `self.LevelCollision.OnComponentEndOverlap`
  (params (OverlappedComponent :type "PrimitiveComponent Object Reference") (OtherActor :type "Actor Object Reference") (OtherComp :type "PrimitiveComponent Object Reference") (OtherBodyIndex :type Integer))
  (cast `/Game/FirstPerson/Blueprints/BP_FirstPersonCharacter` OtherActor)
  (set `self.Itsinthezone` false))

(fn `UserConstructionScript`)