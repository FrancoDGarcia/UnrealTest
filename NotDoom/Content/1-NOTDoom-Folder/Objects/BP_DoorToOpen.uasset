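; BP_DoorToOpen is a sliding door that opens when the first-person character enters its box and closes when they leave.
; If locked, it opens only when the character's KeyEnum contains KeyRequired, otherwise printing a key-needed message.
; A timeline lerps the door's relative location by an offset and reverses to close.
; A dynamic material turns the visor green or red, restoring its original color shortly after exit.
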(event `ColorBacktonormal`
  (`KismetSystemLibrary.Delay` 0.3)
  (`MaterialInstanceDynamic.SetVectorParameterValue` (`self.MyDynamicMaterial`) (`self.Nameofmaterial`) (`self.Value To have`)))

(event `Whatcolorneed`
  (params (`How is the door` :type Boolean))
  (bind _mydynamicmaterial (`self.MyDynamicMaterial`))
  (bind _nameofmaterial (`self.Nameofmaterial`))
  (if `How is the door`
    (`MaterialInstanceDynamic.SetVectorParameterValue` _mydynamicmaterial _nameofmaterial (struct :`G` 0.854167 :`B` 0.022142 :`A` 1.0))
    (else
      (`MaterialInstanceDynamic.SetVectorParameterValue` _mydynamicmaterial _nameofmaterial (struct :`R` 0.854167 :`B` 0.007186 :`A` 1.0)))))

(event `Dynamic`
  (bind _mydynamicmaterial (`self.MyDynamicMaterial`))
  (bind _asbp_first_person_character (cast `/Game/FirstPerson/Blueprints/BP_FirstPersonCharacter` (`GameplayStatics.GetPlayerCharacter` 0)))
  (set `self.As BP First Person Character` _asbp_first_person_character)
  (bind _returnvalue (`KismetMaterialLibrary.CreateDynamicMaterialInstance` "/Game/1-NOTDoom-Folder/DoorwhitkeyDynamicmaterial.DoorwhitkeyDynamicmaterial" "Change"))
  (set `self.MyDynamicMaterial` _returnvalue)
  (`PrimitiveComponent.SetMaterial` (`self.Visor`) 0 (`self.MyDynamicMaterial`))
  (`MaterialInterface.GetBaseMaterial` _mydynamicmaterial)
  (bind _returnvalue_2 (`MaterialInstanceDynamic.K2_GetVectorParameterValue` _mydynamicmaterial (`self.Nameofmaterial`)))
  (set `self.Value To have` _returnvalue_2))

(event `self.ReceiveBeginPlay`
  (`self.Dynamic`)
  (set `self.Ubication Relative` (`SceneComponent.RelativeLocation` (`self.Doorthatneedkey`))))

(event `self.Box.OnComponentBeginOverlap`
  (params (OverlappedComponent :type "PrimitiveComponent Object Reference") (OtherActor :type "Actor Object Reference") (OtherComp :type "PrimitiveComponent Object Reference") (OtherBodyIndex :type Integer) (bFromSweep :type Boolean) (SweepResult :type "HitResult Structure (by ref)"))
  (bind _asbp_first_person_character (cast `/Game/FirstPerson/Blueprints/BP_FirstPersonCharacter` OtherActor))
  (if (`self.ItsLocked`)
    (if (`KismetArrayLibrary.Array_Contains` (`/Game/FirstPerson/Blueprints/BP_FirstPersonCharacter.KeyEnum` _asbp_first_person_character) (`self.KeyRequired`))
      (`self.WhenDoorOpen`)
      (set `self.DoorAlreadyOpen?` true)
      (`self.Whatcolorneed` true :!label _label)
      (else
        (`KismetSystemLibrary.PrintText` "You need the key for this door")
        (`self.Whatcolorneed` false)))
    (else
      (`self.WhenDoorOpen`)
      (set `self.DoorAlreadyOpen?` true)
      (goto _label))))

(event `self.Box.OnComponentEndOverlap`
  (params (OverlappedComponent :type "PrimitiveComponent Object Reference") (OtherActor :type "Actor Object Reference") (OtherComp :type "PrimitiveComponent Object Reference") (OtherBodyIndex :type Integer))
  (cast `/Game/FirstPerson/Blueprints/BP_FirstPersonCharacter` OtherActor)
  (`self.WhenDoorClosed`)
  (set `self.DoorAlreadyOpen?` false)
  (`self.ColorBacktonormal`))

(event `WhenDoorOpen`
  (bind _ubication_relative (`self.Ubication Relative`))
  (bind (_direction _dooropening) (`Timeline|Línea de tiempo_0` :!label _label_2)
    (:`Update`
      (`SceneComponent.K2_SetRelativeLocation` (`self.Doorthatneedkey`) (`KismetMathLibrary.VLerp` _ubication_relative (- _ubication_relative (`self.Positionofmovement`)) _dooropening) false false))))

(event `WhenDoorClosed`
  (goto _label_2 :!via `Reverse`))

(fn `UserConstructionScript`)