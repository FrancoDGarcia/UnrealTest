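; BP_EnemyToSpawn is a placeable spawn point that creates an enemy at its own transform when play begins.
; After a short delay, it converts its enemy-type enum value to a row name and looks it up in the DT_Enemys data table.
; If the row is found, it spawns that row's class, so the enum selection alone decides which enemy appears.
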(event `self.ReceiveBeginPlay`
  (`KismetSystemLibrary.Delay` 0.1)
  (bind _output_get (set `self.Stringtoname` (`|GetEnumeratorNameAsString` (`self.BPEnemyToSpawn`))))
  (set `self.Name` (`KismetStringLibrary.Conv_StringToName` _output_get))
  (bind _returnvalue (`|GetDataTableRow` "/Game/1-NOTDoom-Folder/DataTable/DT_Enemys.DT_Enemys" (`self.Name`))
    (:`then`
      (`|SpawnActorFromClass` (`.ClassToSpawn_35_C25646FE4BE449679597C38FDF88EF30` (break `/Game/1-NOTDoom-Folder/DataTable/Structure_Enemy` _returnvalue)) (`self.GetTransform` self) "Undefined" "OverrideRootScale" null null))))

(fn `UserConstructionScript`)