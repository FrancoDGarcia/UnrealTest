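; BP_Gate is a gate actor that slides its Gate component open and closed.
; BeginPlay stores the component's starting relative location as the closed position.
; OpenDoor and Closethedoor play and reverse one timeline, whose curve lerps the gate between that position and one offset by subtracting MovementPosition.
; The collapse sound call is unconnected, so the gate plays no audio.
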(event `self.ReceiveBeginPlay`
  (set `self.RelativePosition` (`SceneComponent.RelativeLocation` (`self.Gate`))))

(event `OpenDoor`
  (bind _relativeposition (`self.RelativePosition`))
  (bind (_direction _dooropening) (`Timeline|Línea de tiempo_0` :!label _label)
    (:`Update`
      (`SceneComponent.K2_SetRelativeLocation` (`self.Gate`) (`KismetMathLibrary.VLerp` _relativeposition (- _relativeposition (`self.MovementPosition`)) _dooropening) false false))))

(event `Close the door`
  (goto _label :!via `Reverse`))

(fn `UserConstructionScript`)