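; BP_MyMeleeEnemy is a melee enemy that chases the first-person player and deals damage on contact.
; Sighting the player through MyEyes latches a flag that makes Tick call AIMoveTo toward them, and capsule hits damage them.
; Projectile hits on Enemybox reduce health, briefly flashing a dynamic material red on survival or awarding points and destroying the enemy at zero or below.
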(event `AttackedMaterial`
  (bind _my_dynamic_material (`self.My Dynamic Material`))
  (`MaterialInterface.GetBaseMaterial` _my_dynamic_material)
  (bind _returnvalue (`MaterialInstanceDynamic.K2_GetVectorParameterValue` _my_dynamic_material "Change"))
  (set `self.Value to obtain` _returnvalue)
  (`MaterialInstanceDynamic.SetVectorParameterValue` _my_dynamic_material "Change" (struct :`R` 0.854167 :`B` 0.007186 :`A` 1.0))
  (`KismetSystemLibrary.Delay` 0.5)
  (`MaterialInstanceDynamic.SetVectorParameterValue` _my_dynamic_material "Change" (`self.Value to obtain`)))

(event `self.ReceiveBeginPlay`
  (bind _asbp_first_person_character (cast `/Game/FirstPerson/Blueprints/BP_FirstPersonCharacter` (`GameplayStatics.GetPlayerCharacter` 0)))
  (set `self.MyPlayertofollow` _asbp_first_person_character)
  (bind _returnvalue (`KismetMaterialLibrary.CreateDynamicMaterialInstance` "/Game/1-NOTDoom-Folder/EnemyMaterial.EnemyMaterial" "Change"))
  (set `self.My Dynamic Material` _returnvalue)
  (`PrimitiveComponent.SetMaterial` (`self.Enemybox`) 0 (`self.My Dynamic Material`)))

(event `self.ReceiveTick`
  (params (DeltaSeconds :type "Float (single-precision)"))
  (if (`self.I already see the player?`)
    (`|AIMoveTo` self (0.0 0.0 0.0) (`self.MyPlayertofollow`))))

(event `self.MyEyes.OnSeePawn`
  (params (Pawn :type "Pawn Object Reference"))
  (cast `/Game/FirstPerson/Blueprints/BP_FirstPersonCharacter` Pawn)
  (set `self.I already see the player?` true))

(event `self.CapsuleComponent.OnComponentHit`
  (params (HitComponent :type "PrimitiveComponent Object Reference") (OtherActor :type "Actor Object Reference") (OtherComp :type "PrimitiveComponent Object Reference") (NormalImpulse :type "Vector Structure") (Hit :type "HitResult Structure (by ref)"))
  (bind _asbp_first_person_character (cast `/Game/FirstPerson/Blueprints/BP_FirstPersonCharacter` OtherActor))
  (`/Game/FirstPerson/Blueprints/BP_FirstPersonCharacter.PlayerDamaged` _asbp_first_person_character _asbp_first_person_character (`self.Damageofattack`) null null self))

(event `self.Enemybox.OnComponentHit`
  (params (HitComponent :type "PrimitiveComponent Object Reference") (OtherActor :type "Actor Object Reference") (OtherComp :type "PrimitiveComponent Object Reference") (NormalImpulse :type "Vector Structure") (Hit :type "HitResult Structure (by ref)"))
  (bind _asbp_first_person_projectile (cast `/Game/FirstPerson/Blueprints/BP_FirstPersonProjectile` OtherActor))
  (bind _output_get (set `self.MyHealth` (- (`self.MyHealth`) (`/Game/FirstPerson/Blueprints/BP_FirstPersonProjectile.Projectiledamage` _asbp_first_person_projectile))))
  (`/Engine/EditorBlueprintResources/StandardMacros.CompareFloat` _output_get
    (:`>`
      (`self.AttackedMaterial`))
    (:`==`
      (bind _asbp_first_person_character (cast `/Game/FirstPerson/Blueprints/BP_FirstPersonCharacter` (`GameplayStatics.GetPlayerCharacter` 0) :!label _label))
      (`/Game/FirstPerson/Blueprints/BP_FirstPersonCharacter.Points to obtain` _asbp_first_person_character (`self.Points To Give`))
      (`self.K2_DestroyActor`))
    (:`<`
      (goto _label)))
  (`self.K2_DestroyActor` _asbp_first_person_projectile))

(fn `UserConstructionScript`)