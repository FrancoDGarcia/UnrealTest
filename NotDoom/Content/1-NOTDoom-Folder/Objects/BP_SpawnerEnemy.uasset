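; Enemy spawner actor that scatters a random number of enemies inside its Spawner component's bounds.
; BeginPlay rolls a count within min/max limits and spawns a batch immediately, then a short one-shot timer spawns another batch of equal size.
; Each spawn takes a random XY point at the bounds' center height with the spawner's rotation, increments a counter and receives BPtoSpawn after spawning.
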(event `self.ReceiveBeginPlay`
  (set `self.RandomNumber` (`KismetMathLibrary.RandomIntegerInRange` (`self.MinNumberspawn`) (`self.MaxNumberSpawn`)))
  (`KismetSystemLibrary.K2_SetTimerDelegate` (delegate `Enemy`) 0.1)
  (`self.SpawnEnemy`))

(event `Enemy`
  (`self.SpawnEnemy`))

(event `SpawnEnemy`
  (bind _randomnumber (`self.RandomNumber`))
  (bind (_origin _boxextent) (`KismetSystemLibrary.GetComponentBounds` (`self.Spawner`)))
  (for _ (`|MakeArray` _randomnumber)
    (for _ (range 1 (+ _randomnumber 1))
      (if (< 0 _randomnumber)
        (bind _output_get (set `self.EnemySpawnertothemoment` (+ (`self.EnemySpawnertothemoment`) 1)))
        (bind _returnvalue (`|SpawnActorFromClass` "/Game/1-NOTDoom-Folder/Objects/BP_EnemyToSpawn.BP_EnemyToSpawn_C" (`KismetMathLibrary.MakeTransform` (+ (* (`KismetMathLibrary.RandomPointInBoundingBox` _origin _boxextent) (1.0 1.0 0.0)) (* _origin (0.0 0.0 1.0))) (`self.K2_GetActorRotation` self)) "Undefined" "OverrideRootScale" null null))
        (set `/Game/1-NOTDoom-Folder/Objects/BP_EnemyToSpawn.BPEnemyToSpawn` (`self.BPtoSpawn`) _returnvalue)))))

(fn `UserConstructionScript`)