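; BP_Enemy is a first-person game enemy that damages the player on contact.
; A hit on its Enemy1 component calls PlayerDamaged on the first-person character with the enemy's attack damage.
; It caches the player on BeginPlay, but sighting only prints a message, copies a movement variable and adds zero-direction input.
; AI chase and alternative damage chains are left disconnected, so it does not pursue the player.
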(event `self.ReceiveBeginPlay`
  (bind _asbp_first_person_character (cast `/Game/FirstPerson/Blueprints/BP_FirstPersonCharacter` (`GameplayStatics.GetPlayerCharacter` 0)))
  (set `self.MyPlayertofollow` _asbp_first_person_character))

(event `self.Myenemyeyes.OnSeePawn`
  (params (Pawn :type "Pawn Object Reference"))
  (`KismetSystemLibrary.PrintText` "Come on")
  (set `self.Mymovement_0` (`self.Mymovement`))
  (`self.AddMovementInput` (0.0 0.0 0.0)))

(event `self.ReceiveTick`
  (params (DeltaSeconds :type "Float (single-precision)")))

(event `self.Enemy1.OnComponentHit`
  (params (HitComponent :type "PrimitiveComponent Object Reference") (OtherActor :type "Actor Object Reference") (OtherComp :type "PrimitiveComponent Object Reference") (NormalImpulse :type "Vector Structure") (Hit :type "HitResult Structure (by ref)"))
  (bind _asbp_first_person_character (cast `/Game/FirstPerson/Blueprints/BP_FirstPersonCharacter` OtherActor))
  (`/Game/FirstPerson/Blueprints/BP_FirstPersonCharacter.PlayerDamaged` _asbp_first_person_character _asbp_first_person_character (`self.Damageofattack`) null null self))

(event `self.MyCollider.OnComponentHit`
  (params (HitComponent :type "PrimitiveComponent Object Reference") (OtherActor :type "Actor Object Reference") (OtherComp :type "PrimitiveComponent Object Reference") (NormalImpulse :type "Vector Structure") (Hit :type "HitResult Structure (by ref)")))

(event `self.MyCollider.OnComponentBeginOverlap`
  (params (OverlappedComponent :type "PrimitiveComponent Object Reference") (OtherActor :type "Actor Object Reference") (OtherComp :type "PrimitiveComponent Object Reference") (OtherBodyIndex :type Integer) (bFromSweep :type Boolean) (SweepResult :type "HitResult Structure (by ref)")))

(fn `UserConstructionScript`)