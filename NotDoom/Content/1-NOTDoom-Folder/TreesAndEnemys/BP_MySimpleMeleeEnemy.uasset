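; Simple melee enemy that loads stats from DT_Enemys, takes projectile damage with a colour flash, and awards points on death.
; Perception and projectile hits set blackboard range state; the waypoint count is also written there.
; HitEnemy briefly enables a damage box near the player, then waits out a recharge.
; A health widget updates and yaws toward the player every tick; death deactivates the enemy, then destroys it after a delay.
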(event `Attacked`
  (bind _my_dynamic_material (`self.My Dynamic Material`))
  (`MaterialInterface.GetBaseMaterial` _my_dynamic_material)
  (bind _returnvalue (`MaterialInstanceDynamic.K2_GetVectorParameterValue` _my_dynamic_material "Change"))
  (set `self.Value to obtain` _returnvalue)
  (`MaterialInstanceDynamic.SetVectorParameterValue` _my_dynamic_material "Change" (struct :`R` 0.854167 :`B` 0.007186 :`A` 1.0))
  (`KismetSystemLibrary.Delay` 0.5)
  (`MaterialInstanceDynamic.SetVectorParameterValue` _my_dynamic_material "Change" (`self.Value to obtain`)))

(event `self.ReceiveBeginPlay`
  (bind (_nombre _enemyclass _weapontohave _dmg _speed _life _timetoreloadattack _pointstoobtain) (break `/Game/1-NOTDoom-Folder/DataTable/Structure_Enemy` (`self.Structuretohave`)))
  (`BlackboardComponent.SetValueAsInt` (`AIBlueprintHelperLibrary.GetBlackboard` null) "WaypointInTotal" (`KismetArrayLibrary.Array_Length` (`self.Waypoints`)))
  (`/Engine/EditorBlueprintResources/StandardMacros.CompareInt` (`self.Points to Give`)
    (:`==`
      (bind _returnvalue (`|GetDataTableRow` "/Game/1-NOTDoom-Folder/DataTable/DT_Enemys.DT_Enemys" "SimpleMelee")
        (:`then`
          (set `self.Structuretohave` _returnvalue)
          (set `self.DMG` _dmg)
          (set `self.Speed` _speed)
          (bind _output_get (set `self.Life` _life))
          (set `self.Recharge` _timetoreloadattack)
          (set `self.Points to Give` _pointstoobtain)
          (set `self.Initial Life` _output_get)
          (`PrimitiveComponent.SetCollisionEnabled` (`self.Box`) "NoCollision")
          (`self.WidgetLife`)
          (bind _aswgbp_enemy_life (cast `/Game/1-NOTDoom-Folder/Widgets/WGBP_EnemyLife` (`WidgetComponent.GetWidget` (`self.My Widget`)))
            (:`then`
              (set `/Game/1-NOTDoom-Folder/Widgets/WGBP_EnemyLife.MyName` (`KismetTextLibrary.Conv_NameToText` _nombre) _aswgbp_enemy_life))
            (:`CastFailed`
              _))
          (bind _asbp_first_person_character (cast `/Game/FirstPerson/Blueprints/BP_FirstPersonCharacter` (`GameplayStatics.GetPlayerCharacter` 0)))
          (set `self.My Playertofollow` _asbp_first_person_character)
          (bind _returnvalue_2 (`KismetMaterialLibrary.CreateDynamicMaterialInstance` "/Game/1-NOTDoom-Folder/Objects/Materials_and_NiagarraSystem/EnemyMaterial.EnemyMaterial" "Change"))
          (set `self.My Dynamic Material` _returnvalue_2)
          (`PrimitiveComponent.SetMaterial` (`self.Mesh`) 0 (`self.My Dynamic Material`)))))))

(event `WidgetLife`
  (bind _returnvalue (`GameplayStatics.GetPlayerCharacter` 0))
  (bind _my_widget (`self.My Widget`))
  (bind _aswgbp_enemy_life (cast `/Game/1-NOTDoom-Folder/Widgets/WGBP_EnemyLife` (`WidgetComponent.GetWidget` _my_widget)))
  (`ProgressBar.SetPercent` (`/Game/1-NOTDoom-Folder/Widgets/WGBP_EnemyLife.ProgressBar_0` _aswgbp_enemy_life) (/ (`self.Life`) (`self.Initial Life`)))
  (cast `/Game/FirstPerson/Blueprints/BP_FirstPersonCharacter` _returnvalue)
  (`SceneComponent.K2_SetWorldRotation` _my_widget (`KismetMathLibrary.MakeRotator` 0.0 0.0 (.yaw (`KismetMathLibrary.FindLookAtRotation` (`SceneComponent.K2_GetComponentLocation` _my_widget) (`self.K2_GetActorLocation` _returnvalue)))) false false))

(event `self.ReceiveTick`
  (params (DeltaSeconds :type "Float (single-precision)"))
  (`self.WidgetLife`))

(event `self.Box.OnComponentBeginOverlap`
  (params (OverlappedComponent :type "PrimitiveComponent Object Reference") (OtherActor :type "Actor Object Reference") (OtherComp :type "PrimitiveComponent Object Reference") (OtherBodyIndex :type Integer) (bFromSweep :type Boolean) (SweepResult :type "HitResult Structure (by ref)"))
  (bind _asbp_first_person_character (cast `/Game/FirstPerson/Blueprints/BP_FirstPersonCharacter` OtherActor))
  (`/Game/FirstPerson/Blueprints/BP_FirstPersonCharacter.PlayerDamaged` _asbp_first_person_character _asbp_first_person_character (`self.DMG`) null null self)
  (`GameplayStatics.PlaySound2D` (`self.Sound`) 1.0 1.0 0.0 null null))

(event `self.CapsuleComponent.OnComponentHit`
  (params (HitComponent :type "PrimitiveComponent Object Reference") (OtherActor :type "Actor Object Reference") (OtherComp :type "PrimitiveComponent Object Reference") (NormalImpulse :type "Vector Structure") (Hit :type "HitResult Structure (by ref)"))
  (bind _asbp_first_person_projectile (cast `/Game/FirstPerson/Blueprints/BP_FirstPersonProjectile` OtherActor :!label _label))
  (`BlackboardComponent.SetValueAsBool` (`AIBlueprintHelperLibrary.GetBlackboard` null) "IsInRange?" true)
  (bind _output_get (set `self.Life` (- (`self.Life`) (`/Game/FirstPerson/Blueprints/BP_FirstPersonProjectile.Projectiledamage` _asbp_first_person_projectile))))
  (`/Engine/EditorBlueprintResources/StandardMacros.CompareFloat` _output_get
    (:`>`
      (`self.Attacked`)
      (`self.K2_DestroyActor` _asbp_first_person_projectile))
    (:`==`
      (bind _asbp_first_person_character (cast `/Game/FirstPerson/Blueprints/BP_FirstPersonCharacter` (`GameplayStatics.GetPlayerCharacter` 0) :!label _label_2))
      (if (not (`self.Isdead`))
        (`/Game/FirstPerson/Blueprints/BP_FirstPersonCharacter.Points to obtain` _asbp_first_person_character (`self.Points To Give`))
        (set `self.Isdead` true)
        (`ActorComponent.Deactivate` (`self.SK_Blade_FrostGiant`))
        (`/Game/1-NOTDoom-Folder/Objects/CABP_EnemyComponent.DesactivationEvent` (`self.MyEnemyComponent`) (`self.CapsuleComponent`) (`self.CharacterMovement`) "/Game/1-NOTDoom-Folder/ExternalSounds/Male-Death-Sound-2.Male-Death-Sound-2")
        (`self.K2_DestroyActor` _asbp_first_person_projectile)
        (`KismetSystemLibrary.Delay` 15.0)
        (`self.K2_DestroyActor`)))
    (:`<`
      (goto _label_2))))

(event `AttackedBySomething`
  (params (Bullet :type "/Game/FirstPerson/Blueprints/BP_FirstPersonProjectile Object Reference"))
  (goto _label))

(event `self.Perception.OnTargetPerceptionUpdated`
  (params (Actor :type "Actor Object Reference") (Stimulus :type "AIStimulus Structure"))
  (bind _returnvalue (`GameplayStatics.GetPlayerPawn` 0))
  (bind _returnvalue_2 (`AIBlueprintHelperLibrary.GetBlackboard` null))
  (bind _info (`AIPerceptionComponent.GetActorsPerception` (`self.Perception`) _returnvalue))
  (set `self.Successfully Sensed` (`.bSuccessfullySensed` (break `AIStimulus` (`|GetArrayItem` (`.LastSensedStimuli` (break `ActorPerceptionBlueprintInfo` _info))))))
  (if (not (`self.Successfully Sensed`))
    (`KismetSystemLibrary.Delay` 0.2))
  (`BlackboardComponent.SetValueAsBool` _returnvalue_2 "IsInRange?" (`self.Successfully Sensed`))
  (`BlackboardComponent.SetValueAsObject` _returnvalue_2 "Player" _returnvalue))

(event `HitEnemy`
  (bind _box (`self.Box`))
  (if (not (`self.Isdead`))
    (bind _asbp_first_person_character (cast `/Game/FirstPerson/Blueprints/BP_FirstPersonCharacter` (`GameplayStatics.GetPlayerCharacter` 0)))
    (if (== (`self.K2_GetActorLocation` _asbp_first_person_character) (`self.K2_GetActorLocation`) :`ErrorTolerance` 100.0)
      (if (`self.Isattacking`)
        _
        (elif (not (`self.Timetowait`))
          (set `self.Isattacking` true)
          (`KismetSystemLibrary.Delay` 0.15)
          (`PrimitiveComponent.SetCollisionEnabled` _box "QueryAndPhysics")
          (`GameplayStatics.PlaySound2D` "/Game/1-NOTDoom-Folder/ExternalSounds/la-cuchilla_1.la-cuchilla_1" 1.0 1.0 0.0 null null)
          (set `self.Timetowait` true)
          (`KismetSystemLibrary.Delay` 0.4)
          (set `self.Isattacking` false)
          (`PrimitiveComponent.SetCollisionEnabled` _box "NoCollision")
          (`KismetSystemLibrary.Delay` (`self.Recharge`))
          (set `self.Timetowait` false))))))

(fn `UserConstructionScript`)