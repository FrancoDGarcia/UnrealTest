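; BP_SimpleGunEnemy is a ranged enemy that chases and shoots the player, and awards points when killed.
; BeginPlay sets stats from a struct, loaded from DT_Enemys' "SimpleRager" row when PointsToGive is zero.
; Pawn sensing triggers AIMoveTo pursuit and spawns bullets on a recharge delay.
; Projectile hits alert it, reduce life and flash a dynamic material, while Tick updates a player-facing health bar.
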(event `Attacked`
  (bind _my_dynamic_material (`self.My Dynamic Material`))
  (`MaterialInterface.GetBaseMaterial` _my_dynamic_material)
  (bind _returnvalue (`MaterialInstanceDynamic.K2_GetVectorParameterValue` _my_dynamic_material "Change"))
  (set `self.Value to obtain` _returnvalue)
  (`MaterialInstanceDynamic.SetVectorParameterValue` _my_dynamic_material "Change" (struct :`R` 1.0 :`G` 1.0 :`B` 1.0 :`A` 1.0))
  (`KismetSystemLibrary.Delay` 0.5)
  (`MaterialInstanceDynamic.SetVectorParameterValue` _my_dynamic_material "Change" (`self.Value to obtain`)))

(event `self.ReceiveBeginPlay`
  (bind (_nombre _enemyclass _weapontohave _dmg _speed _life _timetoreloadattack _pointstoobtain) (break `/Game/1-NOTDoom-Folder/DataTable/Structure_Enemy` (`self.Structuretohave`)))
  (`/Engine/EditorBlueprintResources/StandardMacros.CompareInt` (`self.Points to Give`)
    (:`>`
      _)
    (:`==`
      (bind _returnvalue (`|GetDataTableRow` "/Game/1-NOTDoom-Folder/DataTable/DT_Enemys.DT_Enemys" "SimpleRager")
        (:`then`
          (set `self.Structuretohave` _returnvalue))))
    (:`<`
      _))
  (set `self.DMG` _dmg)
  (set `self.Speed` _speed)
  (bind _output_get (set `self.Life` _life))
  (set `self.InitialLife` _output_get)
  (set `self.Recharge` _timetoreloadattack)
  (set `self.Points to Give` _pointstoobtain)
  (`self.WidgetLife`)
  (bind _asbp_first_person_character (cast `/Game/FirstPerson/Blueprints/BP_FirstPersonCharacter` (`GameplayStatics.GetPlayerCharacter` 0)))
  (set `self.My Playertofollow` _asbp_first_person_character)
  (bind _returnvalue_2 (`KismetMaterialLibrary.CreateDynamicMaterialInstance` "/Game/1-NOTDoom-Folder/Modelados_y_animaciones/InfinityBladeWarriors/Character/CompleteCharacters/Textures_Materials/CharM_FrostGiant/M_Char_FrostGiant.M_Char_FrostGiant" "Change"))
  (set `self.My Dynamic Material` _returnvalue_2)
  (`PrimitiveComponent.SetMaterial` (`self.Mesh`) 0 (`self.My Dynamic Material`)))

(event `WidgetLife`
  (bind _mywidget (`self.MyWidget`))
  (bind _aswgbp_enemy_life (cast `/Game/1-NOTDoom-Folder/Widgets/WGBP_EnemyLife` (`WidgetComponent.GetWidget` _mywidget)))
  (`ProgressBar.SetPercent` (`/Game/1-NOTDoom-Folder/Widgets/WGBP_EnemyLife.ProgressBar_0` _aswgbp_enemy_life) (/ (`self.Life`) (`self.InitialLife`)))
  (`SceneComponent.K2_SetWorldRotation` _mywidget (`KismetMathLibrary.MakeRotator` 0.0 0.0 (.yaw (`KismetMathLibrary.FindLookAtRotation` (`SceneComponent.K2_GetComponentLocation` _mywidget) (`self.K2_GetActorLocation` (`GameplayStatics.GetPlayerCharacter` 0))))) false false))

(event `self.ReceiveTick`
  (params (DeltaSeconds :type "Float (single-precision)"))
  (bind _capsulecomponent (`self.CapsuleComponent`))
  (`self.WidgetLife`)
  (if (`self.I already see the player?`)
    (`|AIMoveTo` self (0.0 0.0 0.0) (`self.My Playertofollow`) 500.0
      (:`then`
        (`SceneComponent.K2_SetWorldRotation` _capsulecomponent (`KismetMathLibrary.MakeRotator` 0.0 0.0 (.yaw (`KismetMathLibrary.FindLookAtRotation` (`SceneComponent.K2_GetComponentLocation` _capsulecomponent) (`self.K2_GetActorLocation` (`GameplayStatics.GetPlayerCharacter` 0))))) false false)))
    (else
      (`KismetSystemLibrary.Delay` 5.0))))

(event `self.MyEyes.OnSeePawn`
  (params (Pawn :type "Pawn Object Reference"))
  (`|ExecutionSequence`
    (:`then_0`
      (cast `/Game/FirstPerson/Blueprints/BP_FirstPersonCharacter` Pawn
        (:`then`
          (set `self.I already see the player?` true))
        (:`CastFailed`
          (set `self.I Already See The Player?` false))))))

(event `ShootSomething`
  (cast `/Game/FirstPerson/Blueprints/BP_FirstPersonCharacter` (stale `self.Zone To Shoot.OnSeePawn` Pawn))
  (if (`self.I Already See The Player?`) :!label _label
    (if (`self.Timetowait`)
      (`|ExecutionSequence`
        (:`then_0`
          (bind _returnvalue (`|SpawnActorFromClass` "/Game/1-NOTDoom-Folder/Objects/BP_SimpleEnemyBullet.BP_SimpleEnemyBullet_C" (`SceneComponent.K2_GetComponentToWorld` (`self.Sphere`)) "Undefined" "OverrideRootScale" null null))
          (`SceneComponent.K2_SetWorldRotation` (`/Game/1-NOTDoom-Folder/Objects/BP_SimpleEnemyBullet.MyBullet` _returnvalue) (`KismetMathLibrary.MakeRotator` 0.0 0.0 (.yaw (`KismetMathLibrary.FindLookAtRotation` (`SceneComponent.K2_GetComponentLocation` (`self.CapsuleComponent`)) (`self.K2_GetActorLocation` (`GameplayStatics.GetPlayerCharacter` 0))))) false false)
          (set `/Game/1-NOTDoom-Folder/Objects/BP_SimpleEnemyBullet.DMG` (`self.DMG`) _returnvalue)
          (set `self.Timetowait` false)
          (`KismetSystemLibrary.Delay` (`self.Recharge`))
          (set `self.Timetowait` true))))))

(event `self.Zone To Shoot.OnSeePawn`
  (params (Pawn :type "Pawn Object Reference"))
  (cast `/Game/FirstPerson/Blueprints/BP_FirstPersonCharacter` Pawn)
  (goto _label))

(event `Attackedbysomething`
  (params (Person :type "/Game/FirstPerson/Blueprints/BP_FirstPersonProjectile Object Reference")))

(event `self.CapsuleComponent.OnComponentHit`
  (params (HitComponent :type "PrimitiveComponent Object Reference") (OtherActor :type "Actor Object Reference") (OtherComp :type "PrimitiveComponent Object Reference") (NormalImpulse :type "Vector Structure") (Hit :type "HitResult Structure (by ref)"))
  (bind _asbp_first_person_projectile (cast `/Game/FirstPerson/Blueprints/BP_FirstPersonProjectile` OtherActor))
  (set `self.I Already See The Player?` true)
  (bind _output_get (set `self.Life` (- (`self.Life`) (`/Game/FirstPerson/Blueprints/BP_FirstPersonProjectile.Projectiledamage` _asbp_first_person_projectile))))
  (`/Engine/EditorBlueprintResources/StandardMacros.CompareFloat` _output_get
    (:`>`
      (`self.Attacked`))
    (:`==`
      (bind _asbp_first_person_character (cast `/Game/FirstPerson/Blueprints/BP_FirstPersonCharacter` (`GameplayStatics.GetPlayerCharacter` 0) :!label _label_2))
      (`/Game/FirstPerson/Blueprints/BP_FirstPersonCharacter.Points to obtain` _asbp_first_person_character (`self.Points To Give`))
      (`self.K2_DestroyActor`))
    (:`<`
      (goto _label_2)))
  (`self.K2_DestroyActor` _asbp_first_person_projectile))

(event `self.Mesh.OnComponentBeginOverlap`
  (params (OverlappedComponent :type "PrimitiveComponent Object Reference") (OtherActor :type "Actor Object Reference") (OtherComp :type "PrimitiveComponent Object Reference") (OtherBodyIndex :type Integer) (bFromSweep :type Boolean) (SweepResult :type "HitResult Structure (by ref)")))

(fn `UserConstructionScript`)