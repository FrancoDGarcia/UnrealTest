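; BP_DoorToOpen is a sliding door that opens when the first-person character enters its trigger box.
; If locked, it requires KeyRequired in the character's KeyEnum, otherwise it prints a message that a key is needed.
; A timeline lerps the door mesh's relative location by Positionofmovement from its starting position.
; Leaving the box reverses the timeline only for locked doors, so unlocked doors stay open.
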(event `self.ReceiveBeginPlay`
  (set `self.Ubication Relative` (`SceneComponent.RelativeLocation` (`self.Doorthatneedkey`))))

(event `self.Box.OnComponentBeginOverlap`
  (params (OverlappedComponent :type "PrimitiveComponent Object Reference") (OtherActor :type "Actor Object Reference") (OtherComp :type "PrimitiveComponent Object Reference") (OtherBodyIndex :type Integer) (bFromSweep :type Boolean) (SweepResult :type "HitResult Structure (by ref)"))
  (bind _asbp_first_person_character (cast `/Game/FirstPerson/Blueprints/BP_FirstPersonCharacter` OtherActor))
  (if (`self.ItsLocked`)
    (if (`KismetArrayLibrary.Array_Contains` (`/Game/FirstPerson/Blueprints/BP_FirstPersonCharacter.KeyEnum` _asbp_first_person_character) (`self.KeyRequired`))
      (`self.WhenDoorOpen`)
      (set `self.DoorAlreadyOpen?` true)
      (else
        (`KismetSystemLibrary.PrintText` "You need the key for this door")))
    (else
      (`self.WhenDoorOpen`)
      (set `self.DoorAlreadyOpen?` true))))

(event `self.Box.OnComponentEndOverlap`
  (params (OverlappedComponent :type "PrimitiveComponent Object Reference") (OtherActor :type "Actor Object Reference") (OtherComp :type "PrimitiveComponent Object Reference") (OtherBodyIndex :type Integer))
  (cast `/Game/FirstPerson/Blueprints/BP_FirstPersonCharacter` OtherActor)
  (if (`self.ItsLocked`)
    (`self.WhenDoorClosed`)
    (set `self.DoorAlreadyOpen?` false)))

(event `WhenDoorOpen`
  (bind _ubication_relative (`self.Ubication Relative`))
  (bind (_direction _dooropening) (`Timeline|Línea de tiempo_0` :!label _label)
    (:`Update`
      (`SceneComponent.K2_SetRelativeLocation` (`self.Doorthatneedkey`) (`KismetMathLibrary.VLerp` _ubication_relative (- _ubication_relative (`self.Positionofmovement`)) _dooropening) false false))))

(event `WhenDoorClosed`
  (goto _label :!via `Reverse`))

(fn `UserConstructionScript`)